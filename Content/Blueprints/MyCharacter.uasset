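; MyCharacter is a first-person player character with torso turning controlled separately through a TorsoTurn input axis.
; On BeginPlay the camera snaps to the mesh's ViewPoint socket, and each Tick sets its world rotation to the actor's rotation, independent of torso rotation.
; Tick also prints torso pitch and yaw and draws a debug sphere.
; The Delete key triggers an orientation and position reset.
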(event `self.ReceiveBeginPlay`
  (`SceneComponent.K2_AttachTo` (`self.FirstPersonCameraComponent`) (`self.Mesh`) "ViewPoint" "SnapToTarget" true))

(event `self.ReceiveTick`
  (params (DeltaSeconds :type "Float (single-precision)"))
  (`SceneComponent.SetWorldRotation` (`self.FirstPersonCameraComponent`) (`self.K2_GetActorRotation`) false)
  (bind _returnvalue (`self.GetTorsoRotation`))
  (`KismetSystemLibrary.PrintString` null (`KismetStringLibrary.Conv_RotatorToString` (`KismetMathLibrary.MakeRot` (.pitch _returnvalue) (.yaw _returnvalue))))
  (`KismetSystemLibrary.DrawDebugSphere` null))

(event `InputAxis|TorsoTurn`
  (params (AxisValue :type "Float (single-precision)"))
  (`self.AddTorsoYawInput` AxisValue))

(event `Key|Delete`
  (:`Pressed`
    (`HeadMountedDisplayFunctionLibrary.ResetOrientationAndPosition` 0.0)))

(fn `UserConstructionScript`)